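; BP_GraphPoint is a clickable point actor in a pathfinding graph.
; On BeginPlay it caches the first BP_Manager found in the level.
; A left click on its Box sets this point as the manager's EndPoint, while any other mouse button passes it to the manager's AddPoint.
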(event OnClicked(Box)
  (params (TouchedComponent :type Primitive%20Component%20Object%20Reference) (ButtonPressed :type Key%20Structure :default "None"))
  (bind _manager (Variables|Default|GetManager))
  (if (== ButtonPressed "LeftMouseButton")
    (Variables|/Script/MPIA_IA.Manager|SetEndPoint _manager self)
    (else
      (Class|Manager|AddPoint _manager self))))

(event EventBeginPlay
  (bind _outactors (Actor|GetAllActorsOfClass "/Game/Pathfinding/BP_Manager.BP_Manager_C"))
  (Variables|Default|SetManager (Utilities|Array|Get(acopy) _outactors)))

(event Collision|EventActorBeginOverlap
  (params (OtherActor :type Actor%20Object%20Reference)))

(event EventTick
  (params (DeltaSeconds :type Float%20%28single-precision%29)))

(fn ConstructionScript)